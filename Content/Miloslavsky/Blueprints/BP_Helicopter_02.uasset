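; Player-flyable helicopter that a first-person character enters and exits through possession, attachment and Enhanced Input context swaps.
; Tick spools RPM and engine sound until takeoff, then interpolates input into swept movement, tilt and yaw while spinning rotors.
; A delayed downward trace clears the airborne state on landing.
; Also handles timeline-animated doors and trunk on number keys, mouse look, cabin/external camera toggle and material color theming.
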(event Input|EnhancedActionEvents|EnhancedInputActionIA_Move
  (params (ActionValue :type Vector%202D%20Structure) (ElapsedSeconds :type Float%20%28double-precision%29) (TriggeredSeconds :type Float%20%28double-precision%29) (InputAction :type Input%20Action%20Object%20Reference :default "/Game/Miloslavsky/Input/Actions/IA_Move.IA_Move"))
  ;[0 0 0] Forward-Backward movement
  ;;[1 0 0.08333] IA_Move
  (:Triggered
    (Variables|Default|SetFrontBackAxis (.x ActionValue) :!label _label))
  (:Completed
    (goto _label)))

(event Input|EnhancedActionEvents|EnhancedInputActionIA_ChangeCamera
  (params (ActionValue :type Boolean) (ElapsedSeconds :type Float%20%28double-precision%29) (TriggeredSeconds :type Float%20%28double-precision%29) (InputAction :type Input%20Action%20Object%20Reference :default "/Game/Miloslavsky/Input/Actions/IA_ChangeCamera.IA_ChangeCamera"))
  ;[0 0 0] ChangeCamera
  ;;[1 0 0.08333] IA_ChangeCamera
  (:Triggered
    (Utilities|FlowControl|FlipFlop
      (:A
        (Variables|Default|SetActiveCamera (Variables|Default|GetCameraCabin))
        (Components|Activation|Deactivate (Variables|Default|GetCamera))
        (Components|Activation|Activate (Variables|Default|GetCameraCabin) false))
      (:B
        (Variables|Default|SetActiveCamera (Variables|Default|GetCamera))
        (Components|Activation|Deactivate (Variables|Default|GetCameraCabin))
        (Components|Activation|Activate (Variables|Default|GetCamera) false)))))

(event Input|EnhancedActionEvents|EnhancedInputActionIA_Interaction
  (params (ActionValue :type Boolean) (ElapsedSeconds :type Float%20%28double-precision%29) (TriggeredSeconds :type Float%20%28double-precision%29) (InputAction :type Input%20Action%20Object%20Reference :default "/Game/Miloslavsky/Input/Actions/IA_Interaction.IA_Interaction"))
  (bind _self self)
  (bind _returnvalue (Pawn|GetController _self))
  ;[0 0.3333 1] Exit helicopter
  ;;[1 0 0.08333] IA_Interact
  (:Triggered
    (Transformation|DetachFromActor (Variables|Default|GetDriver) "KeepWorld" "KeepWorld" "KeepWorld")
    (Transformation|SetActorLocation (Variables|Default|GetDriver) (Transformation|GetWorldLocation (Variables|Default|GetEnterBoxLeft)) false false)
    (bind _asplayer_controller (Utilities|Casting|CastToPlayerController _returnvalue))
    (Utilities|IsValid (PlayerController|LocalPlayerSubsystems|GetEnhancedInputLocalPlayerSubsystem _asplayer_controller)
      (:Is%20Valid
        (Input|RemoveMappingContext (PlayerController|LocalPlayerSubsystems|GetEnhancedInputLocalPlayerSubsystem _asplayer_controller) "/Game/Miloslavsky/Input/IMC_Helicopter.IMC_Helicopter" "(bIgnoreAllPressedKeysUntilRelease=True,bForceImmediately=False)")
        (Input|AddMappingContext (PlayerController|LocalPlayerSubsystems|GetEnhancedInputLocalPlayerSubsystem _asplayer_controller) "/Game/Miloslavsky/Input/IMC_FP.IMC_FP" 0 "(bIgnoreAllPressedKeysUntilRelease=True,bForceImmediately=False)")
        (bind _asbp_first_person_character (Utilities|Casting|CastToBP_FirstPersonCharacter (Variables|Default|GetDriver)))
        (Default|EnableCapsuleCollision _asbp_first_person_character true)
        (Pawn|Possess _returnvalue _asbp_first_person_character)))))

(event Input|EnhancedActionEvents|EnhancedInputActionIA_YawRotation
  (params (ActionValue :type Float%20%28double-precision%29) (ElapsedSeconds :type Float%20%28double-precision%29) (TriggeredSeconds :type Float%20%28double-precision%29) (InputAction :type Input%20Action%20Object%20Reference :default "/Game/Miloslavsky/Input/Actions/IA_YawRotation.IA_YawRotation"))
  ;[0 0 0] Yaw movement
  ;;[1 0 0.08333] Yaw rotation
  (:Triggered
    (Variables|Default|SetYaw (!= 0.0 ActionValue))
    (Variables|Default|SetYawRotSpeed (Math|Interpolation|FInterpTo (Variables|Default|GetYawRotSpeed) (* ActionValue (Variables|Default|GetYawRotSpeedFactor)) (Utilities|Time|GetWorldDeltaSeconds) 2.0)))
  (:Completed
    (Variables|Default|SetYawRotSpeed 0.0)))

(event Input|EnhancedActionEvents|EnhancedInputActionIA_UpDown
  (params (ActionValue :type Float%20%28double-precision%29) (ElapsedSeconds :type Float%20%28double-precision%29) (TriggeredSeconds :type Float%20%28double-precision%29) (InputAction :type Input%20Action%20Object%20Reference :default "/Game/Miloslavsky/Input/Actions/IA_UpDown.IA_UpDown"))
  ;[0 0 0] Up-Down movement
  ;;[1 0 0.08333] IA_UpDown
  (:Triggered
    (Variables|Default|SetUpDownAxis ActionValue :!label _label))
  (:Completed
    (goto _label)))

(event Input|EnhancedActionEvents|EnhancedInputActionIA_Look
  (params (ActionValue :type Vector%202D%20Structure) (ElapsedSeconds :type Float%20%28double-precision%29) (TriggeredSeconds :type Float%20%28double-precision%29) (InputAction :type Input%20Action%20Object%20Reference :default "/Game/Miloslavsky/Input/Actions/IA_Look.IA_Look"))
  (bind _springarm (Variables|Default|GetSpringArm))
  (bind _relativerotation (Variables|/Script/Engine.SceneComponent|GetRelativeRotation _springarm))
  ;[0 0 0] Mouse look
  ;;[1 0 0.08333] input action mouse Look
  (:Triggered
    (Transformation|AddRelativeRotation (Variables|Default|GetSpringArm) (Math|Rotator|MakeRotator 0.0 (* (.x ActionValue) -1.0) 0.0) false false)
    (Transformation|SetRelativeRotation _springarm (Math|Rotator|MakeRotator (.roll _relativerotation) (Math|Float|Clamp(Float) (.pitch _relativerotation) -75.0 75.0) (.yaw _relativerotation)) false false)))

(event Input|EnhancedActionEvents|EnhancedInputActionIA_Move
  (params (ActionValue :type Vector%202D%20Structure) (ElapsedSeconds :type Float%20%28double-precision%29) (TriggeredSeconds :type Float%20%28double-precision%29) (InputAction :type Input%20Action%20Object%20Reference :default "/Game/Miloslavsky/Input/Actions/IA_Move.IA_Move"))
  ;[0 0 0] Right-Left movement
  ;;[1 0 0.08333] IA_RightLeft
  (:Triggered
    (Variables|Default|SetSidesAxes (.y ActionValue) :!label _label))
  (:Completed
    (goto _label)))

(event Input|EnhancedActionEvents|EnhancedInputActionIA_Look
  (params (ActionValue :type Vector%202D%20Structure) (ElapsedSeconds :type Float%20%28double-precision%29) (TriggeredSeconds :type Float%20%28double-precision%29) (InputAction :type Input%20Action%20Object%20Reference :default "/Game/Miloslavsky/Input/Actions/IA_Look.IA_Look"))
  ;[0 0 0] Mouse look
  ;;[1 0 0.08333] input action mouse Look
  (:Triggered
    (Transformation|AddRelativeRotation (Variables|Default|GetSpringArm) (Math|Rotator|MakeRotator 0.0 0.0 (.y ActionValue)) false false)))

(event EventOnInteraction
  (params (Interactor :type Pawn%20Object%20Reference))
  ;[0 0.3333 1] Enter helicopter
  ;;[1 0 0.08333] OnInteraction
  (bind _output_get (Variables|Default|SetDriver Interactor))
  (bind _asbp_first_person_character (Utilities|Casting|CastToBP_FirstPersonCharacter _output_get))
  (Default|EnableCapsuleCollision _asbp_first_person_character false)
  (bind _asplayer_controller (Utilities|Casting|CastToPlayerController (Pawn|GetController _asbp_first_person_character)))
  (Utilities|IsValid (PlayerController|LocalPlayerSubsystems|GetEnhancedInputLocalPlayerSubsystem _asplayer_controller)
    (:Is%20Valid
      ;;[0.2 0.2 0.2] Switch inputs to helicopter's
      (Input|RemoveMappingContext (PlayerController|LocalPlayerSubsystems|GetEnhancedInputLocalPlayerSubsystem _asplayer_controller) "/Game/Miloslavsky/Input/IMC_FP.IMC_FP" "(bIgnoreAllPressedKeysUntilRelease=True,bForceImmediately=False)")
      (Input|AddMappingContext (PlayerController|LocalPlayerSubsystems|GetEnhancedInputLocalPlayerSubsystem _asplayer_controller) "/Game/Miloslavsky/Input/IMC_Helicopter.IMC_Helicopter" 0 "(bIgnoreAllPressedKeysUntilRelease=True,bForceImmediately=False)")
      (Pawn|Possess (Pawn|GetController (Variables|Default|GetDriver)) self)
      (Transformation|AttachActorToActor (Variables|Default|GetDriver) self "plot_seat" "SnapToTarget" "SnapToTarget" "SnapToTarget" true)
      ;;[0.2 0.2 0.2] Detach from attach parent (ex. Yacht)
      (Transformation|DetachFromActor "KeepWorld" "KeepWorld" "KeepWorld"))))

(event EventTick
  (params (DeltaSeconds :type Float%20%28single-precision%29))
  (bind _returnvalue (Transformation|GetActorRotation))
  (bind _helicopter_sound (Variables|Default|Gethelicopter_Sound))
  ;[0 0 0] Helicopter movement
  ;;[1 0 0.08333] Tick
  ;[0 1 0.5] Update axes
  (Utilities|FlowControl|Sequence
    (:then_0
      ;[0 0 0] Forward-Backward movement
      (Variables|Default|SetFBSpeed (Math|Interpolation|FInterpTo (Variables|Default|GetFBSpeed) (* (Variables|Default|GetFrontBackAxis) (Variables|Default|GetFBSpeedFactor)) (Utilities|Time|GetWorldDeltaSeconds) 2.0)))
    (:then_1
      ;[0 0 0] Right-Left movement
      (Variables|Default|SetRLSpeed (Math|Interpolation|FInterpTo (Variables|Default|GetRLSpeed) (* (Variables|Default|GetSidesAxes) (Variables|Default|GetRLSpeedFactor)) (Utilities|Time|GetWorldDeltaSeconds) 2.0)))
    (:then_2
      (if (Variables|Default|GetInAir)
        (Variables|Default|SetUDSpeed (Math|Interpolation|FInterpTo (Variables|Default|GetUDSpeed) (* (Variables|Default|GetUpDownAxis) (Variables|Default|GetUDSpeedFactor)) (Utilities|Time|GetWorldDeltaSeconds) 2.0))
        (else
          (Variables|Default|SetRPM (Math|Float|Clamp(Float) (+ (* (Variables|Default|GetUpDownAxis) 3.0) (Variables|Default|GetRPM)) 0.0 1.5e+03))
          (Variables|Default|SetInAir (> (Variables|Default|GetRPM) 1e+03))
          (Audio|Parameter|SetFloatParameter (Variables|Default|Gethelicopter_Sound) "Volume" (/ (Variables|Default|GetRPM) 8e+02) :!class /Script/Engine.AudioComponent)
          (Audio|Parameter|SetFloatParameter (Variables|Default|Gethelicopter_Sound) "Pitch" (/ (Variables|Default|GetRPM) 1e+03) :!class /Script/Engine.AudioComponent)
          (if (> (Variables|Default|GetRPM) 0.0)
            (Components|Activation|Activate _helicopter_sound false)
            (else
              (Components|Activation|Deactivate _helicopter_sound))))))
    (:then_3
      (if (Variables|Default|GetInAir)
        ;;[0 0 0] Rotors rotation
        ;;;[0.1349 1 0] вот с этой гниды клинит камеру из кабины. Переписать
        (Variables|Default|SetBladeRotatorSpeed (Math|Interpolation|FInterpTo (Variables|Default|GetBladeRotatorSpeed) (Variables|Default|GetRPM) (Utilities|Time|GetWorldDeltaSeconds) 2.0))
        (Transformation|AddRelativeRotation (Variables|Default|Getmain_rotor) (Math|Rotator|MakeRotator 0.0 0.0 (* (Variables|Default|GetBladeRotatorSpeed) (* (Utilities|Time|GetWorldDeltaSeconds) (Variables|Default|GetBladeSpeed)))) false false)
        (Transformation|AddRelativeRotation (Variables|Default|Getrear_rotor) (Math|Rotator|MakeRotator 0.0 0.0 (* (* (Variables|Default|GetBladeRotatorSpeed) (* (Utilities|Time|GetWorldDeltaSeconds) (Variables|Default|GetBladeSpeed))) 0.5)) false false)
        (bind _output_get (Variables|Default|SetDeltaLoaction (* (+ (Math|Vector|ProjectVectorontoPlane (+ (* (Transformation|GetActorForwardVector) (Math|Conversions|ToVector(Float) (Variables|Default|GetFBSpeed))) (* (Transformation|GetActorRightVector) (Math|Conversions|ToVector(Float) (Variables|Default|GetRLSpeed)))) "0, 0,1.000000") (* (Transformation|GetActorUpVector) (Math|Conversions|ToVector(Float) (Variables|Default|GetUDSpeed)))) (Math|Conversions|ToVector(Float) (Utilities|Time|GetWorldDeltaSeconds)))))
        (Transformation|AddActorWorldOffset _output_get true)
        (if (Variables|Default|GetYaw)
          ;;[0 0 0] йав
          (Transformation|SetActorRotation (Math|Rotator|MakeRotator (.roll _returnvalue) (.pitch _returnvalue) (+ (.yaw _returnvalue) (* (Variables|Default|GetYawRotSpeed) (Utilities|Time|GetWorldDeltaSeconds)))))
          (else
            ;;[0 0 0] тангаж мув
            (Transformation|SetActorRotation (Math|Rotator|MakeRotator (* (Variables|Default|GetRLSpeed) (Variables|Default|GetRLSpeedToRoll)) (* (Variables|Default|GetFBSpeed) (Variables|Default|GetFBSpeedToPitch)) (+ (.yaw (Transformation|GetActorRotation)) (Variables|Default|GetRLSpeed))))
            (Utilities|FlowControl|Delay 0.5)
            (CallFunction|Ground)))
        (else
          ;;[0 1 0.2401] Non-flying mode (вертолет не в воздухе не позволяет выйти из кабины - переписать через Enhanced Input)
          (Variables|Default|SetBladeRotatorSpeed (Math|Interpolation|FInterpTo (Variables|Default|GetBladeRotatorSpeed) (Variables|Default|GetRPM) (Utilities|Time|GetWorldDeltaSeconds) 2.0))
          (Transformation|AddRelativeRotation (Variables|Default|Getmain_rotor) (Math|Rotator|MakeRotator 0.0 0.0 (* (Variables|Default|GetBladeRotatorSpeed) (* (Utilities|Time|GetWorldDeltaSeconds) (Variables|Default|GetBladeSpeed)))) false false)
          (Transformation|AddRelativeRotation (Variables|Default|Getrear_rotor) (Math|Rotator|MakeRotator 0.0 0.0 (* (* (Variables|Default|GetBladeRotatorSpeed) (* (Utilities|Time|GetWorldDeltaSeconds) (Variables|Default|GetBladeSpeed))) 0.5)) false false))))))

(event Input|KeyboardEvents|5
  (params (Key :type Key%20Structure :default "None"))
  ;[0 0 0] Door Open and Close
  (:Pressed
    (Utilities|FlowControl|FlipFlop
      (:A
        (bind (_direction _moveforward_track _moveback_track) (Timeline|Timeline_4 PlayFromStart)
          (:Update
            (Transformation|SetRelativeRotation (Variables|Default|GetTrunk_R) (Math|Rotator|MakeRotator 0.0 0.0 (* _moveback_track -6e+01)) false false)
            (Transformation|SetRelativeRotation (Variables|Default|GetTrunk_L) (Math|Rotator|MakeRotator 0.0 0.0 (* _moveforward_track 6e+01)) false false))))
      (:B
        (Timeline|Timeline_4 Reverse)))))

(event Input|KeyboardEvents|NumPadFour
  (params (Key :type Key%20Structure :default "None"))
  ;[0 0 0] Door Open and Close
  (:Pressed
    (Utilities|FlowControl|FlipFlop
      (:A
        (bind (_direction _moveforward_track _moveback_track) (Timeline|Timeline_3 PlayFromStart)
          (:Update
            (Transformation|SetRelativeLocation (Variables|Default|Getback_door_L) (Math|Vector|MakeVector (* _moveback_track -152.0) (* _moveforward_track -7.5) 0.0) false false))))
      (:B
        (Timeline|Timeline_3 Reverse)))))

(event Input|KeyboardEvents|NumPadFive
  (params (Key :type Key%20Structure :default "None"))
  ;[0 0 0] Door Open and Close
  (:Pressed
    (Utilities|FlowControl|FlipFlop
      (:A
        (bind (_direction _moveforward_track _moveback_track) (Timeline|Timeline_4 PlayFromStart)
          (:Update
            (Transformation|SetRelativeRotation (Variables|Default|GetTrunk_R) (Math|Rotator|MakeRotator 0.0 0.0 (* _moveback_track -6e+01)) false false)
            (Transformation|SetRelativeRotation (Variables|Default|GetTrunk_L) (Math|Rotator|MakeRotator 0.0 0.0 (* _moveforward_track 6e+01)) false false))))
      (:B
        (Timeline|Timeline_4 Reverse)))))

(event Input|KeyboardEvents|NumPadOne
  (params (Key :type Key%20Structure :default "None"))
  ;[0 0 0] Door Open and Close
  (:Pressed
    (Utilities|FlowControl|FlipFlop
      (:A
        (bind _door_front_r (Timeline|Timeline_0 PlayFromStart)
          (:Update
            (Transformation|SetRelativeRotation (Variables|Default|Getfront_door_R) (Math|Rotator|MakeRotator 0.0 0.0 (* _door_front_r -6e+01)) false false))))
      (:B
        (Timeline|Timeline_0 Reverse)))))

(event Input|KeyboardEvents|1
  (params (Key :type Key%20Structure :default "None"))
  ;[0 0 0] Door Open and Close
  (:Pressed
    (Utilities|FlowControl|FlipFlop
      (:A
        (bind _door_front_r (Timeline|Timeline_0 PlayFromStart)
          (:Update
            (Transformation|SetRelativeRotation (Variables|Default|Getfront_door_R) (Math|Rotator|MakeRotator 0.0 0.0 (* _door_front_r -6e+01)) false false))))
      (:B
        (Timeline|Timeline_0 Reverse)))))

(event Input|KeyboardEvents|NumPadTwo
  (params (Key :type Key%20Structure :default "None"))
  ;[0 0 0] Door Open and Close
  (:Pressed
    (Utilities|FlowControl|FlipFlop
      (:A
        (bind _door_front_r (Timeline|Timeline_1 PlayFromStart)
          (:Update
            (Transformation|SetRelativeRotation (Variables|Default|Getfront_door_L) (Math|Rotator|MakeRotator 0.0 0.0 (* _door_front_r 6e+01)) false false))))
      (:B
        (Timeline|Timeline_1 Reverse)))))

(event Input|KeyboardEvents|2
  (params (Key :type Key%20Structure :default "None"))
  ;[0 0 0] Door Open and Close
  (:Pressed
    (Utilities|FlowControl|FlipFlop
      (:A
        (bind _door_front_r (Timeline|Timeline_1 PlayFromStart)
          (:Update
            (Transformation|SetRelativeRotation (Variables|Default|Getfront_door_L) (Math|Rotator|MakeRotator 0.0 0.0 (* _door_front_r 6e+01)) false false))))
      (:B
        (Timeline|Timeline_1 Reverse)))))

(event Input|KeyboardEvents|NumPadThree
  (params (Key :type Key%20Structure :default "None"))
  ;[0 0 0] Door Open and Close
  (:Pressed
    (Utilities|FlowControl|FlipFlop
      (:A
        (bind (_direction _moveforward_track _moveback_track) (Timeline|Timeline_2 PlayFromStart)
          (:Update
            (Transformation|SetRelativeLocation (Variables|Default|Getback_door_R) (Math|Vector|MakeVector (* _moveback_track -152.0) (* _moveforward_track 7.5) 0.0) false false))))
      (:B
        (Timeline|Timeline_2 Reverse)))))

(event Input|KeyboardEvents|3
  (params (Key :type Key%20Structure :default "None"))
  ;[0 0 0] Door Open and Close
  (:Pressed
    (Utilities|FlowControl|FlipFlop
      (:A
        (bind (_direction _moveforward_track _moveback_track) (Timeline|Timeline_2 PlayFromStart)
          (:Update
            (Transformation|SetRelativeLocation (Variables|Default|Getback_door_R) (Math|Vector|MakeVector (* _moveback_track -152.0) (* _moveforward_track 7.5) 0.0) false false))))
      (:B
        (Timeline|Timeline_2 Reverse)))))

(event Input|KeyboardEvents|4
  (params (Key :type Key%20Structure :default "None"))
  ;[0 0 0] Door Open and Close
  (:Pressed
    (Utilities|FlowControl|FlipFlop
      (:A
        (bind (_direction _moveforward_track _moveback_track) (Timeline|Timeline_3 PlayFromStart)
          (:Update
            (Transformation|SetRelativeLocation (Variables|Default|Getback_door_L) (Math|Vector|MakeVector (* _moveback_track -152.0) (* _moveforward_track -7.5) 0.0) false false))))
      (:B
        (Timeline|Timeline_3 Reverse)))))

(fn ConstructionScript)

(fn Ground
  (bind _body (Variables|Default|Getbody))
  (bind _returnvalue (Transformation|GetWorldLocation _body))
  (bind _returnvalue_2 (Collision|LineTraceByChannel _returnvalue (+ (* (Math|Vector|GetUpVector (Transformation|GetWorldRotation _body)) -1e+02) _returnvalue) "TraceTypeQuery1" false 0 "None"))
  (if _returnvalue_2
    (Variables|Default|SetInAir false)))

(fn SetTheme
  (params (Color :type Linear%20Color%20Structure))
  (bind _body (Variables|Default|Getbody))
  (bind _rear_rotor (Variables|Default|Getrear_rotor))
  (bind _main_rotor (Variables|Default|Getmain_rotor))
  (Utilities|SetThemeColortoMaterial _body 2 "Color_02" Color
    (:Output
      (Utilities|SetThemeColortoMaterial _body 2 "Color_03" Color
        (:Output
          (Utilities|SetThemeColortoMaterial _rear_rotor 0 "Color_01" Color
            (:Output
              (Utilities|SetThemeColortoMaterial _rear_rotor 0 "Color_02" Color
                (:Output
                  (Utilities|SetThemeColortoMaterial (Variables|Default|Getback_door_L) 3 "Color_02" Color
                    (:Output
                      (Utilities|SetThemeColortoMaterial (Variables|Default|Getback_door_R) 3 "Color_02" Color
                        (:Output
                          (Utilities|SetThemeColortoMaterial (Variables|Default|GetTrunk_L) 1 "Color_02" Color
                            (:Output
                              (Utilities|SetThemeColortoMaterial (Variables|Default|GetTrunk_R) 1 "Color_02" Color
                                (:Output
                                  (Utilities|SetThemeColortoMaterial _main_rotor 1 "Color_01" Color
                                    (:Output
                                      (Utilities|SetThemeColortoMaterial _main_rotor 1 "Color_02" Color))))))))))))))))))))
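; Configurable door that rotates or slides open and closed on trigger overlap (unless use-only), interaction, activation or automatically at begin play.
; Timelines lerp the mesh transform and reverse to close, with optional delayed auto-close.
; Rotating doors pick swing direction from the dot product of the chosen forward axis and the direction to the activator.
; The construction script applies mesh, open speed, starting state and trigger zone size.
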(event Custom|CloseRotation
  ;[0 0 0] Open rotation
  (bind _alpha (Timeline|TL_Rorate Reverse)
    (:Update
      (Transformation|SetRelativeRotation (Variables|Default|GetMeshDoor) (Math|Rotator|MakeRotator (.x (Math|Vector|Lerp(Vector) (Variables|Default|GetInitRotation) (select (>= (Variables|Default|GetDot) 0.0) (+ (Variables|Default|GetInitRotation) (Variables|DOORPARAMETERS|GetDistance)) (- (Variables|Default|GetInitRotation) (Variables|DOORPARAMETERS|GetDistance))) _alpha)) (.y (Math|Vector|Lerp(Vector) (Variables|Default|GetInitRotation) (select (>= (Variables|Default|GetDot) 0.0) (+ (Variables|Default|GetInitRotation) (Variables|DOORPARAMETERS|GetDistance)) (- (Variables|Default|GetInitRotation) (Variables|DOORPARAMETERS|GetDistance))) _alpha)) (.z (Math|Vector|Lerp(Vector) (Variables|Default|GetInitRotation) (select (>= (Variables|Default|GetDot) 0.0) (+ (Variables|Default|GetInitRotation) (Variables|DOORPARAMETERS|GetDistance)) (- (Variables|Default|GetInitRotation) (Variables|DOORPARAMETERS|GetDistance))) _alpha))) false false))
    (:Finished
      ;;[0.2 0.2 0.2] Autoclose
      (Utilities|AutoCloseOption (Variables|Default|GetTL_Rorate))
      (CallFunction|CloseRotation))))

(event Custom|CloseSliding
  ;[0 0 0] Open slide
  (bind _alpha (Timeline|TL_Slide Reverse)
    (:Update
      (Transformation|SetRelativeLocation (Variables|Default|GetMeshDoor) (Math|Vector|Lerp(Vector) (Variables|Default|GetInitialLocation) (Variables|DOORPARAMETERS|GetDistance) _alpha) false false))
    (:Finished
      ;;[0.2 0.2 0.2] Autoclose
      (Utilities|AutoCloseOption (Variables|Default|GetTL_Slide))
      (CallFunction|CloseSliding))))

(event EventOnActivation
  (params (Activator :type Actor%20Object%20Reference) (Preceding :type Actor%20Object%20Reference) (ActivationType :type Byte :default 0))
  ;[1 0 0.08333] OnActivation
  (switch Utilities|FlowControl|Switch|SwitchonBPE_Door_Type (Variables|DOORPARAMETERS|GetDoorType)
    (:NewEnumerator0
      ;[0 0 0] Open rotation
      (if (Variables|Default|GetIsOpen)
        (Variables|Default|SetIsOpen false)
        (CallFunction|CloseRotation)
        (else
          (Variables|Default|SetIsOpen true)
          (bind _dot (Utilities|GetDotPlayerandDoor (Variables|Default|GetActivator))
            (:Out
              (Variables|Default|SetDot _dot)
              (bind _alpha (Timeline|TL_Rorate Play)
                (:Update
                  (Transformation|SetRelativeRotation (Variables|Default|GetMeshDoor) (Math|Rotator|MakeRotator (.x (Math|Vector|Lerp(Vector) (Variables|Default|GetInitRotation) (select (>= (Variables|Default|GetDot) 0.0) (+ (Variables|Default|GetInitRotation) (Variables|DOORPARAMETERS|GetDistance)) (- (Variables|Default|GetInitRotation) (Variables|DOORPARAMETERS|GetDistance))) _alpha)) (.y (Math|Vector|Lerp(Vector) (Variables|Default|GetInitRotation) (select (>= (Variables|Default|GetDot) 0.0) (+ (Variables|Default|GetInitRotation) (Variables|DOORPARAMETERS|GetDistance)) (- (Variables|Default|GetInitRotation) (Variables|DOORPARAMETERS|GetDistance))) _alpha)) (.z (Math|Vector|Lerp(Vector) (Variables|Default|GetInitRotation) (select (>= (Variables|Default|GetDot) 0.0) (+ (Variables|Default|GetInitRotation) (Variables|DOORPARAMETERS|GetDistance)) (- (Variables|Default|GetInitRotation) (Variables|DOORPARAMETERS|GetDistance))) _alpha))) false false))
                (:Finished
                  ;;[0.2 0.2 0.2] Autoclose
                  (Utilities|AutoCloseOption (Variables|Default|GetTL_Rorate))
                  (CallFunction|CloseRotation))))))))
    (:NewEnumerator1
      ;[0 0 0] Open slide
      (if (Variables|Default|GetIsOpen)
        (Variables|Default|SetIsOpen false)
        (CallFunction|CloseSliding)
        (else
          (Variables|Default|SetIsOpen true)
          (bind _alpha_2 (Timeline|TL_Slide Play)
            (:Update
              (Transformation|SetRelativeLocation (Variables|Default|GetMeshDoor) (Math|Vector|Lerp(Vector) (Variables|Default|GetInitialLocation) (Variables|DOORPARAMETERS|GetDistance) _alpha_2) false false))
            (:Finished
              ;;[0.2 0.2 0.2] Autoclose
              (Utilities|AutoCloseOption (Variables|Default|GetTL_Slide))
              (CallFunction|CloseSliding))))))))

(event Collision|EventActorBeginOverlap
  (params (OtherActor :type Actor%20Object%20Reference))
  ;[1 0 0.08333] BeginOverlap
  (Variables|Default|SetActivator OtherActor)
  (if (not (Variables|DOORPARAMETERS|GetUseOnly))
    (switch Utilities|FlowControl|Switch|SwitchonBPE_Door_Type (Variables|DOORPARAMETERS|GetDoorType)
      (:NewEnumerator0
        ;[0 0 0] Open rotation
        (if (Variables|Default|GetIsOpen)
          (Variables|Default|SetIsOpen false)
          (CallFunction|CloseRotation)
          (else
            (Variables|Default|SetIsOpen true)
            (bind _dot (Utilities|GetDotPlayerandDoor (Variables|Default|GetActivator))
              (:Out
                (Variables|Default|SetDot _dot)
                (bind _alpha (Timeline|TL_Rorate Play)
                  (:Update
                    (Transformation|SetRelativeRotation (Variables|Default|GetMeshDoor) (Math|Rotator|MakeRotator (.x (Math|Vector|Lerp(Vector) (Variables|Default|GetInitRotation) (select (>= (Variables|Default|GetDot) 0.0) (+ (Variables|Default|GetInitRotation) (Variables|DOORPARAMETERS|GetDistance)) (- (Variables|Default|GetInitRotation) (Variables|DOORPARAMETERS|GetDistance))) _alpha)) (.y (Math|Vector|Lerp(Vector) (Variables|Default|GetInitRotation) (select (>= (Variables|Default|GetDot) 0.0) (+ (Variables|Default|GetInitRotation) (Variables|DOORPARAMETERS|GetDistance)) (- (Variables|Default|GetInitRotation) (Variables|DOORPARAMETERS|GetDistance))) _alpha)) (.z (Math|Vector|Lerp(Vector) (Variables|Default|GetInitRotation) (select (>= (Variables|Default|GetDot) 0.0) (+ (Variables|Default|GetInitRotation) (Variables|DOORPARAMETERS|GetDistance)) (- (Variables|Default|GetInitRotation) (Variables|DOORPARAMETERS|GetDistance))) _alpha))) false false))
                  (:Finished
                    ;;[0.2 0.2 0.2] Autoclose
                    (Utilities|AutoCloseOption (Variables|Default|GetTL_Rorate))
                    (CallFunction|CloseRotation))))))))
      (:NewEnumerator1
        ;[0 0 0] Open slide
        (if (Variables|Default|GetIsOpen)
          (Variables|Default|SetIsOpen false)
          (CallFunction|CloseSliding)
          (else
            (Variables|Default|SetIsOpen true)
            (bind _alpha_2 (Timeline|TL_Slide Play)
              (:Update
                (Transformation|SetRelativeLocation (Variables|Default|GetMeshDoor) (Math|Vector|Lerp(Vector) (Variables|Default|GetInitialLocation) (Variables|DOORPARAMETERS|GetDistance) _alpha_2) false false))
              (:Finished
                ;;[0.2 0.2 0.2] Autoclose
                (Utilities|AutoCloseOption (Variables|Default|GetTL_Slide))
                (CallFunction|CloseSliding)))))))))

(event EventBeginPlay
  ;[1 0 0.08333] Begin play
  (if (Variables|DOORPARAMETERS|GetAutoOpen)
    (Utilities|FlowControl|Delay (Variables|DOORPARAMETERS|GetDelayBeforeOpen))
    (switch Utilities|FlowControl|Switch|SwitchonBPE_Door_Type (Variables|DOORPARAMETERS|GetDoorType)
      (:NewEnumerator0
        ;[0 0 0] Open rotation
        (if (Variables|Default|GetIsOpen)
          (Variables|Default|SetIsOpen false)
          (CallFunction|CloseRotation)
          (else
            (Variables|Default|SetIsOpen true)
            (bind _dot (Utilities|GetDotPlayerandDoor (Variables|Default|GetActivator))
              (:Out
                (Variables|Default|SetDot _dot)
                (bind _alpha (Timeline|TL_Rorate Play)
                  (:Update
                    (Transformation|SetRelativeRotation (Variables|Default|GetMeshDoor) (Math|Rotator|MakeRotator (.x (Math|Vector|Lerp(Vector) (Variables|Default|GetInitRotation) (select (>= (Variables|Default|GetDot) 0.0) (+ (Variables|Default|GetInitRotation) (Variables|DOORPARAMETERS|GetDistance)) (- (Variables|Default|GetInitRotation) (Variables|DOORPARAMETERS|GetDistance))) _alpha)) (.y (Math|Vector|Lerp(Vector) (Variables|Default|GetInitRotation) (select (>= (Variables|Default|GetDot) 0.0) (+ (Variables|Default|GetInitRotation) (Variables|DOORPARAMETERS|GetDistance)) (- (Variables|Default|GetInitRotation) (Variables|DOORPARAMETERS|GetDistance))) _alpha)) (.z (Math|Vector|Lerp(Vector) (Variables|Default|GetInitRotation) (select (>= (Variables|Default|GetDot) 0.0) (+ (Variables|Default|GetInitRotation) (Variables|DOORPARAMETERS|GetDistance)) (- (Variables|Default|GetInitRotation) (Variables|DOORPARAMETERS|GetDistance))) _alpha))) false false))
                  (:Finished
                    ;;[0.2 0.2 0.2] Autoclose
                    (Utilities|AutoCloseOption (Variables|Default|GetTL_Rorate))
                    (CallFunction|CloseRotation))))))))
      (:NewEnumerator1
        ;[0 0 0] Open slide
        (if (Variables|Default|GetIsOpen)
          (Variables|Default|SetIsOpen false)
          (CallFunction|CloseSliding)
          (else
            (Variables|Default|SetIsOpen true)
            (bind _alpha_2 (Timeline|TL_Slide Play)
              (:Update
                (Transformation|SetRelativeLocation (Variables|Default|GetMeshDoor) (Math|Vector|Lerp(Vector) (Variables|Default|GetInitialLocation) (Variables|DOORPARAMETERS|GetDistance) _alpha_2) false false))
              (:Finished
                ;;[0.2 0.2 0.2] Autoclose
                (Utilities|AutoCloseOption (Variables|Default|GetTL_Slide))
                (CallFunction|CloseSliding)))))))))

(event EventOnInteraction
  (params (Interactor :type Pawn%20Object%20Reference))
  ;[1 0 0.08333] OnInteract
  (switch Utilities|FlowControl|Switch|SwitchonBPE_Door_Type (Variables|DOORPARAMETERS|GetDoorType)
    (:NewEnumerator0
      ;[0 0 0] Open rotation
      (if (Variables|Default|GetIsOpen)
        (Variables|Default|SetIsOpen false)
        (CallFunction|CloseRotation)
        (else
          (Variables|Default|SetIsOpen true)
          (bind _dot (Utilities|GetDotPlayerandDoor (Variables|Default|GetActivator))
            (:Out
              (Variables|Default|SetDot _dot)
              (bind _alpha (Timeline|TL_Rorate Play)
                (:Update
                  (Transformation|SetRelativeRotation (Variables|Default|GetMeshDoor) (Math|Rotator|MakeRotator (.x (Math|Vector|Lerp(Vector) (Variables|Default|GetInitRotation) (select (>= (Variables|Default|GetDot) 0.0) (+ (Variables|Default|GetInitRotation) (Variables|DOORPARAMETERS|GetDistance)) (- (Variables|Default|GetInitRotation) (Variables|DOORPARAMETERS|GetDistance))) _alpha)) (.y (Math|Vector|Lerp(Vector) (Variables|Default|GetInitRotation) (select (>= (Variables|Default|GetDot) 0.0) (+ (Variables|Default|GetInitRotation) (Variables|DOORPARAMETERS|GetDistance)) (- (Variables|Default|GetInitRotation) (Variables|DOORPARAMETERS|GetDistance))) _alpha)) (.z (Math|Vector|Lerp(Vector) (Variables|Default|GetInitRotation) (select (>= (Variables|Default|GetDot) 0.0) (+ (Variables|Default|GetInitRotation) (Variables|DOORPARAMETERS|GetDistance)) (- (Variables|Default|GetInitRotation) (Variables|DOORPARAMETERS|GetDistance))) _alpha))) false false))
                (:Finished
                  ;;[0.2 0.2 0.2] Autoclose
                  (Utilities|AutoCloseOption (Variables|Default|GetTL_Rorate))
                  (CallFunction|CloseRotation))))))))
    (:NewEnumerator1
      ;[0 0 0] Open slide
      (if (Variables|Default|GetIsOpen)
        (Variables|Default|SetIsOpen false)
        (CallFunction|CloseSliding)
        (else
          (Variables|Default|SetIsOpen true)
          (bind _alpha_2 (Timeline|TL_Slide Play)
            (:Update
              (Transformation|SetRelativeLocation (Variables|Default|GetMeshDoor) (Math|Vector|Lerp(Vector) (Variables|Default|GetInitialLocation) (Variables|DOORPARAMETERS|GetDistance) _alpha_2) false false))
            (:Finished
              ;;[0.2 0.2 0.2] Autoclose
              (Utilities|AutoCloseOption (Variables|Default|GetTL_Slide))
              (CallFunction|CloseSliding))))))))

(fn ConstructionScript
  (bind _meshdoor (Variables|Default|GetMeshDoor))
  (bind _triggerzone (Variables|DOORPARAMETERS|GetTriggerZone))
  (bind _triggerbox (Variables|Default|GetTriggerBox))
  (bind _cubeillusionary (Variables|Default|GetCubeIllusionary))
  (bind _timetoopen (Variables|DOORPARAMETERS|GetTimeToOpen))
  (bind _distance (Variables|DOORPARAMETERS|GetDistance))
  (bind _triggerzonecoords (Variables|DOORPARAMETERS|GetTriggerZoneCoords))
  (bind _returnvalue (Transformation|GetRelativeTransform _meshdoor))
  (bind _returnvalue_2 (/ 1.0 _timetoopen))
  (Utilities|FlowControl|Sequence
    (:then_0
      ;[0 0 0] Set door mesh
      (Components|StaticMesh|SetStaticMesh (Variables|Default|GetMeshDoor) (Variables|DOORPARAMETERS|GetNewDoorMesh))
      ;[0 0 0] Set time to open
      (Components|Timeline|SetPlayRate (Variables|Default|GetTL_Rorate) _returnvalue_2)
      (Components|Timeline|SetPlayRate (Variables|Default|GetTL_Slide) _returnvalue_2)
      ;[0 0 0] Set Initial location and rotation
      (Variables|Default|SetInitialLocation (.location _returnvalue))
      (Variables|Default|SetInitRotation (Math|Vector|MakeVector (.roll (.rotation _returnvalue)) (.pitch (.rotation _returnvalue)) (.yaw (.rotation _returnvalue))))
      ;[0 0 0] Set axis for rotation/slide
      (Variables|Default|SetForwardDirection (Utilities|Select :Index (Variables|DOORPARAMETERS|GetForwardAxis) :NewEnumerator0 "1.000000,0.000000,0.000000" :NewEnumerator1 "0.000000,1.000000,0.000000" :NewEnumerator2 "0.000000,0.000000,1.000000"))
      ;[0 0 0] Starts open?
      (if (Variables|DOORPARAMETERS|GetStartsOpen)
        (switch Utilities|FlowControl|Switch|SwitchonBPE_Door_Type (Variables|DOORPARAMETERS|GetDoorType)
          (:NewEnumerator0
            (Transformation|SetRelativeRotation (Variables|Default|GetMeshDoor) (Math|Rotator|MakeRotator (.x _distance) (.y _distance) (.z _distance)) false false)
            (Components|Timeline|SetNewTime (Variables|Default|GetTL_Rorate) 1.0))
          (:NewEnumerator1
            (Transformation|SetRelativeLocation (Variables|Default|GetMeshDoor) (Variables|DOORPARAMETERS|GetDistance) false false)
            (Components|Timeline|SetNewTime (Variables|Default|GetTL_Slide) 1.0)))
        (Variables|Default|SetIsOpen true)))
    (:then_1
      ;[0 0 0] Trigger collision
      (Components|Box|SetBoxExtent _triggerbox (/ _triggerzone 2) true)
      (Transformation|SetRelativeLocation _triggerbox _triggerzonecoords false false)
      (Transformation|SetRelativeScale3D _cubeillusionary (/ _triggerzone 100))
      (Transformation|SetRelativeLocation _cubeillusionary _triggerzonecoords false false))))
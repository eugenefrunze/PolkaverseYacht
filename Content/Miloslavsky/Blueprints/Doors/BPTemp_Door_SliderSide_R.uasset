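; Sliding door that toggles open and closed along a spline, triggered by actor overlap (unless UseOnly), activation or interaction.
; A timeline, its play rate scaled by Speed over spline length, drives the mesh's world location and optionally rotation along the path.
; AutoClose reverses it after a delay if fully open.
; The construction script sets the mesh and takes the spline from MovingPath, falling back to its own.
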(event Custom|MoveReverse
  (bind _trainmesh (Variables|Default|GetTrainMesh))
  (bind _pathspline (Variables|Default|GetPathSpline))
  (bind _relativescale3d (Variables|/Script/Engine.SceneComponent|GetRelativeScale3D _trainmesh))
  ;[0 0 0] Move along spline
  (bind _alpha (Timeline|TL_MovingAloneSpline Reverse)
    (:Update
      (Transformation|SetWorldLocationAndRotation (Variables|Default|GetTrainMesh) (.location (select (Variables|Default|GetLocationOnly) (Math|Transform|MakeTransform (Spline|GetLocationatDistanceAlongSpline _pathspline (Math|Float|Lerp 0.0 (Spline|GetSplineLength (Variables|Default|GetPathSpline)) _alpha) "World") (Variables|/Script/Engine.SceneComponent|GetRelativeRotation _trainmesh) _relativescale3d) (Math|Transform|MakeTransform (Spline|GetLocationatDistanceAlongSpline _pathspline (Math|Float|Lerp 0.0 (Spline|GetSplineLength (Variables|Default|GetPathSpline)) _alpha) "World") (Spline|GetRotationatDistanceAlongSpline _pathspline (Math|Float|Lerp 0.0 (Spline|GetSplineLength (Variables|Default|GetPathSpline)) _alpha) "Local") _relativescale3d))) (.rotation (select (Variables|Default|GetLocationOnly) (Math|Transform|MakeTransform (Spline|GetLocationatDistanceAlongSpline _pathspline (Math|Float|Lerp 0.0 (Spline|GetSplineLength (Variables|Default|GetPathSpline)) _alpha) "World") (Variables|/Script/Engine.SceneComponent|GetRelativeRotation _trainmesh) _relativescale3d) (Math|Transform|MakeTransform (Spline|GetLocationatDistanceAlongSpline _pathspline (Math|Float|Lerp 0.0 (Spline|GetSplineLength (Variables|Default|GetPathSpline)) _alpha) "World") (Spline|GetRotationatDistanceAlongSpline _pathspline (Math|Float|Lerp 0.0 (Spline|GetSplineLength (Variables|Default|GetPathSpline)) _alpha) "Local") _relativescale3d))) false false))
    (:Finished
      ;;[0.2 0.2 0.2] AutoClose
      (if (Variables|Default|GetAutoClose)
        (Utilities|FlowControl|Delay (Variables|Default|GetDelayBeforeClose))
        (if (== (Components|Timeline|GetPlaybackPosition (Variables|Default|GetTL_MovingAloneSpline)) 1.0)
          (Variables|Default|SetisOpen false)
          (CallFunction|MoveReverse))))))

(event EventOnActivation
  (params (Activator :type Actor%20Object%20Reference) (Preceding :type Actor%20Object%20Reference))
  (bind _trainmesh (Variables|Default|GetTrainMesh))
  (bind _pathspline (Variables|Default|GetPathSpline))
  (bind _relativescale3d (Variables|/Script/Engine.SceneComponent|GetRelativeScale3D _trainmesh))
  ;[1 0 0.08333] OnActivation
  ;[0 0 0] Set play rate to move with certain speed
  (Components|Timeline|SetPlayRate (Variables|Default|GetTL_MovingAloneSpline) (/ (Variables|Default|GetSpeed) (/ (Spline|GetSplineLength (Variables|Default|GetPathSpline)) 1e+02)))
  ;[0 0 0] Move along spline
  (if (Variables|Default|GetisOpen)
    (Variables|Default|SetisOpen false)
    (CallFunction|MoveReverse)
    (else
      (Variables|Default|SetisOpen true)
      (bind _alpha (Timeline|TL_MovingAloneSpline Play)
        (:Update
          (Transformation|SetWorldLocationAndRotation (Variables|Default|GetTrainMesh) (.location (select (Variables|Default|GetLocationOnly) (Math|Transform|MakeTransform (Spline|GetLocationatDistanceAlongSpline _pathspline (Math|Float|Lerp 0.0 (Spline|GetSplineLength (Variables|Default|GetPathSpline)) _alpha) "World") (Variables|/Script/Engine.SceneComponent|GetRelativeRotation _trainmesh) _relativescale3d) (Math|Transform|MakeTransform (Spline|GetLocationatDistanceAlongSpline _pathspline (Math|Float|Lerp 0.0 (Spline|GetSplineLength (Variables|Default|GetPathSpline)) _alpha) "World") (Spline|GetRotationatDistanceAlongSpline _pathspline (Math|Float|Lerp 0.0 (Spline|GetSplineLength (Variables|Default|GetPathSpline)) _alpha) "Local") _relativescale3d))) (.rotation (select (Variables|Default|GetLocationOnly) (Math|Transform|MakeTransform (Spline|GetLocationatDistanceAlongSpline _pathspline (Math|Float|Lerp 0.0 (Spline|GetSplineLength (Variables|Default|GetPathSpline)) _alpha) "World") (Variables|/Script/Engine.SceneComponent|GetRelativeRotation _trainmesh) _relativescale3d) (Math|Transform|MakeTransform (Spline|GetLocationatDistanceAlongSpline _pathspline (Math|Float|Lerp 0.0 (Spline|GetSplineLength (Variables|Default|GetPathSpline)) _alpha) "World") (Spline|GetRotationatDistanceAlongSpline _pathspline (Math|Float|Lerp 0.0 (Spline|GetSplineLength (Variables|Default|GetPathSpline)) _alpha) "Local") _relativescale3d))) false false))
        (:Finished
          ;;[0.2 0.2 0.2] AutoClose
          (if (Variables|Default|GetAutoClose)
            (Utilities|FlowControl|Delay (Variables|Default|GetDelayBeforeClose))
            (if (== (Components|Timeline|GetPlaybackPosition (Variables|Default|GetTL_MovingAloneSpline)) 1.0)
              (Variables|Default|SetisOpen false)
              (CallFunction|MoveReverse))))))))

(event EventOnInteraction
  (params (Interactor :type Pawn%20Object%20Reference))
  (bind _trainmesh (Variables|Default|GetTrainMesh))
  (bind _pathspline (Variables|Default|GetPathSpline))
  (bind _relativescale3d (Variables|/Script/Engine.SceneComponent|GetRelativeScale3D _trainmesh))
  ;[1 0 0.08333] OnInteraction
  ;[0 0 0] Set play rate to move with certain speed
  (Components|Timeline|SetPlayRate (Variables|Default|GetTL_MovingAloneSpline) (/ (Variables|Default|GetSpeed) (/ (Spline|GetSplineLength (Variables|Default|GetPathSpline)) 1e+02)))
  ;[0 0 0] Move along spline
  (if (Variables|Default|GetisOpen)
    (Variables|Default|SetisOpen false)
    (CallFunction|MoveReverse)
    (else
      (Variables|Default|SetisOpen true)
      (bind _alpha (Timeline|TL_MovingAloneSpline Play)
        (:Update
          (Transformation|SetWorldLocationAndRotation (Variables|Default|GetTrainMesh) (.location (select (Variables|Default|GetLocationOnly) (Math|Transform|MakeTransform (Spline|GetLocationatDistanceAlongSpline _pathspline (Math|Float|Lerp 0.0 (Spline|GetSplineLength (Variables|Default|GetPathSpline)) _alpha) "World") (Variables|/Script/Engine.SceneComponent|GetRelativeRotation _trainmesh) _relativescale3d) (Math|Transform|MakeTransform (Spline|GetLocationatDistanceAlongSpline _pathspline (Math|Float|Lerp 0.0 (Spline|GetSplineLength (Variables|Default|GetPathSpline)) _alpha) "World") (Spline|GetRotationatDistanceAlongSpline _pathspline (Math|Float|Lerp 0.0 (Spline|GetSplineLength (Variables|Default|GetPathSpline)) _alpha) "Local") _relativescale3d))) (.rotation (select (Variables|Default|GetLocationOnly) (Math|Transform|MakeTransform (Spline|GetLocationatDistanceAlongSpline _pathspline (Math|Float|Lerp 0.0 (Spline|GetSplineLength (Variables|Default|GetPathSpline)) _alpha) "World") (Variables|/Script/Engine.SceneComponent|GetRelativeRotation _trainmesh) _relativescale3d) (Math|Transform|MakeTransform (Spline|GetLocationatDistanceAlongSpline _pathspline (Math|Float|Lerp 0.0 (Spline|GetSplineLength (Variables|Default|GetPathSpline)) _alpha) "World") (Spline|GetRotationatDistanceAlongSpline _pathspline (Math|Float|Lerp 0.0 (Spline|GetSplineLength (Variables|Default|GetPathSpline)) _alpha) "Local") _relativescale3d))) false false))
        (:Finished
          ;;[0.2 0.2 0.2] AutoClose
          (if (Variables|Default|GetAutoClose)
            (Utilities|FlowControl|Delay (Variables|Default|GetDelayBeforeClose))
            (if (== (Components|Timeline|GetPlaybackPosition (Variables|Default|GetTL_MovingAloneSpline)) 1.0)
              (Variables|Default|SetisOpen false)
              (CallFunction|MoveReverse))))))))

(event Collision|EventActorBeginOverlap
  (params (OtherActor :type Actor%20Object%20Reference))
  (bind _trainmesh (Variables|Default|GetTrainMesh))
  (bind _pathspline (Variables|Default|GetPathSpline))
  (bind _relativescale3d (Variables|/Script/Engine.SceneComponent|GetRelativeScale3D _trainmesh))
  ;[1 0 0.08333] Overlap
  (if (not (Variables|Default|GetUseOnly))
    ;[0 0 0] Set play rate to move with certain speed
    (Components|Timeline|SetPlayRate (Variables|Default|GetTL_MovingAloneSpline) (/ (Variables|Default|GetSpeed) (/ (Spline|GetSplineLength (Variables|Default|GetPathSpline)) 1e+02)))
    ;[0 0 0] Move along spline
    (if (Variables|Default|GetisOpen)
      (Variables|Default|SetisOpen false)
      (CallFunction|MoveReverse)
      (else
        (Variables|Default|SetisOpen true)
        (bind _alpha (Timeline|TL_MovingAloneSpline Play)
          (:Update
            (Transformation|SetWorldLocationAndRotation (Variables|Default|GetTrainMesh) (.location (select (Variables|Default|GetLocationOnly) (Math|Transform|MakeTransform (Spline|GetLocationatDistanceAlongSpline _pathspline (Math|Float|Lerp 0.0 (Spline|GetSplineLength (Variables|Default|GetPathSpline)) _alpha) "World") (Variables|/Script/Engine.SceneComponent|GetRelativeRotation _trainmesh) _relativescale3d) (Math|Transform|MakeTransform (Spline|GetLocationatDistanceAlongSpline _pathspline (Math|Float|Lerp 0.0 (Spline|GetSplineLength (Variables|Default|GetPathSpline)) _alpha) "World") (Spline|GetRotationatDistanceAlongSpline _pathspline (Math|Float|Lerp 0.0 (Spline|GetSplineLength (Variables|Default|GetPathSpline)) _alpha) "Local") _relativescale3d))) (.rotation (select (Variables|Default|GetLocationOnly) (Math|Transform|MakeTransform (Spline|GetLocationatDistanceAlongSpline _pathspline (Math|Float|Lerp 0.0 (Spline|GetSplineLength (Variables|Default|GetPathSpline)) _alpha) "World") (Variables|/Script/Engine.SceneComponent|GetRelativeRotation _trainmesh) _relativescale3d) (Math|Transform|MakeTransform (Spline|GetLocationatDistanceAlongSpline _pathspline (Math|Float|Lerp 0.0 (Spline|GetSplineLength (Variables|Default|GetPathSpline)) _alpha) "World") (Spline|GetRotationatDistanceAlongSpline _pathspline (Math|Float|Lerp 0.0 (Spline|GetSplineLength (Variables|Default|GetPathSpline)) _alpha) "Local") _relativescale3d))) false false))
          (:Finished
            ;;[0.2 0.2 0.2] AutoClose
            (if (Variables|Default|GetAutoClose)
              (Utilities|FlowControl|Delay (Variables|Default|GetDelayBeforeClose))
              (if (== (Components|Timeline|GetPlaybackPosition (Variables|Default|GetTL_MovingAloneSpline)) 1.0)
                (Variables|Default|SetisOpen false)
                (CallFunction|MoveReverse)))))))))

(fn ConstructionScript
  (bind _movingpath (Variables|Default|GetMovingPath))
  ;[0 0 0] Set train model
  (Components|StaticMesh|SetStaticMesh (Variables|Default|GetTrainMesh) (Variables|Default|GetNewTrainMesh))
  ;[0 0 0] Set path spline from BP_PathSpline object
  (Utilities|IsValid _movingpath
    (:Is%20Valid
      (Variables|Default|SetPathSpline (Variables|/Game/Miloslavsky/Blueprints/BP_PathSpline.BP_PathSpline_C|GetSpline_Path _movingpath)))
    (:Is%20Not%20Valid
      (Variables|Default|SetPathSpline (Variables|Default|GetSplinePathBase)))))
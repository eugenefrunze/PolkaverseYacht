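; BP_Button is a button actor built around a resizable trigger zone; its event graph has no active logic, so it defines no press behavior here.
; The construction script clamps the TriggerZone size to a per-axis minimum, then sizes both TriggerBox and the CubeIllusionary component to match.
; Both components are offset by half the size, so the zone extends from the actor origin as a corner rather than being centered.
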(event EventBeginPlay)

(event Collision|EventActorBeginOverlap
  (params (OtherActor :type Actor%20Object%20Reference)))

(event EventTick
  (params (DeltaSeconds :type Float%20%28single-precision%29)))

(fn ConstructionScript
  (bind _triggerbox (Variables|Default|GetTriggerBox))
  ;[0.2 0.2 0.2] set minimal sizes
  (Variables|Default|SetTriggerZone (Math|Vector|MakeVector (Math|Float|Max(Float) (.X (Math|Vector|BreakVector (Variables|Default|GetTriggerZone))) 1e+02) (Math|Float|Max(Float) (.Y (Math|Vector|BreakVector (Variables|Default|GetTriggerZone))) 1e+02) (Math|Float|Max(Float) (.Z (Math|Vector|BreakVector (Variables|Default|GetTriggerZone))) 1e+02)))
  ;[0.2 0.2 0.2] set trigger box sizes
  (Components|Box|SetBoxExtent (Variables|Default|GetTriggerBox) (/ (Variables|Default|GetTriggerZone) 2.0) true)
  (Transformation|SetRelativeScale3D (Variables|Default|GetCubeIllusionary) (Math|Vector|MakeVector (/ (.x (Variables|Default|GetTriggerZone)) 1e+02) (/ (.y (Variables|Default|GetTriggerZone)) 1e+02) (/ (.z (Variables|Default|GetTriggerZone)) 1e+02)))
  ;[0.2 0.2 0.2] set non-center location and scale
  (Transformation|SetRelativeLocation _triggerbox (/ (Variables|Default|GetTriggerZone) 2.0) false false)
  (Transformation|SetRelativeLocation (Variables|Default|GetCubeIllusionary) (/ (Variables|Default|GetTriggerZone) 2.0) false false)
  (Transformation|SetRelativeScale3D _triggerbox (Math|Vector|MakeVector 1.0 1.0 1.0)))
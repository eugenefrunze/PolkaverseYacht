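; Trigger volume that sends an activation message to a target actor implementing BPI_IInteract.
; Pawn overlap or OnActivation starts it unless UseOnly is set, in which case only OnInteraction does.
; All three events share one path using the overlap's OtherActor as Pawn, with a delay and optional one-shot guard.
; The construction script clamps the zone's minimum size and fits the box and preview cube from a corner origin.
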(event EventOnActivation
  (params (Activator :type Actor%20Object%20Reference) (Preceding :type Actor%20Object%20Reference) (ActivationType :type Byte :default 0))
  ;[1 0 0.08333] On Activation
  (if (not (Variables|Default|GetUseOnly))
    (if (not (and (Variables|Default|GetOnce) (Variables|Default|GetAlreadyWorked)))
      (if (Utilities|DoesObjectImplementInterface (Variables|Default|GetTargetToActivate) "/Game/Miloslavsky/Blueprints/BPI_IInteract.BPI_IInteract_C")
        (bind _aspawn (Utilities|Casting|CastToPawn (stale Collision|EventActorBeginOverlap OtherActor)))
        (Utilities|FlowControl|Delay (Variables|Default|GetDelayBeforeTrigger))
        ;[0.2 0.2 0.2] OnActivation on target
        (Class|BPIIInteract|OnActivation(Message) (Variables|Default|GetTargetToActivate) self _aspawn (Variables|Default|GetActivationType))
        (Variables|Default|SetAlreadyWorked true)))))

(event EventOnInteraction
  (params (Interactor :type Pawn%20Object%20Reference))
  ;[1 0 0.08333] On Interaction
  (if (Variables|Default|GetUseOnly)
    (if (not (and (Variables|Default|GetOnce) (Variables|Default|GetAlreadyWorked)))
      (if (Utilities|DoesObjectImplementInterface (Variables|Default|GetTargetToActivate) "/Game/Miloslavsky/Blueprints/BPI_IInteract.BPI_IInteract_C")
        (bind _aspawn (Utilities|Casting|CastToPawn (stale Collision|EventActorBeginOverlap OtherActor)))
        (Utilities|FlowControl|Delay (Variables|Default|GetDelayBeforeTrigger))
        ;[0.2 0.2 0.2] OnActivation on target
        (Class|BPIIInteract|OnActivation(Message) (Variables|Default|GetTargetToActivate) self _aspawn (Variables|Default|GetActivationType))
        (Variables|Default|SetAlreadyWorked true)))))

(event Collision|EventActorBeginOverlap
  (params (OtherActor :type Actor%20Object%20Reference))
  ;[1 0 0.08333] Begin overlap
  (if (not (Variables|Default|GetUseOnly))
    (if (not (and (Variables|Default|GetOnce) (Variables|Default|GetAlreadyWorked)))
      (if (Utilities|DoesObjectImplementInterface (Variables|Default|GetTargetToActivate) "/Game/Miloslavsky/Blueprints/BPI_IInteract.BPI_IInteract_C")
        (bind _aspawn (Utilities|Casting|CastToPawn OtherActor))
        (Utilities|FlowControl|Delay (Variables|Default|GetDelayBeforeTrigger))
        ;[0.2 0.2 0.2] OnActivation on target
        (Class|BPIIInteract|OnActivation(Message) (Variables|Default|GetTargetToActivate) self _aspawn (Variables|Default|GetActivationType))
        (Variables|Default|SetAlreadyWorked true)))))

(fn ConstructionScript
  (bind _triggerbox (Variables|Default|GetTriggerBox))
  ;[0.2 0.2 0.2] set minimal sizes
  (Variables|Default|SetTriggerZone (Math|Vector|MakeVector (Math|Float|Max(Float) (.X (Math|Vector|BreakVector (Variables|Default|GetTriggerZone))) 1e+02) (Math|Float|Max(Float) (.Y (Math|Vector|BreakVector (Variables|Default|GetTriggerZone))) 1e+02) (Math|Float|Max(Float) (.Z (Math|Vector|BreakVector (Variables|Default|GetTriggerZone))) 1e+02)))
  ;[0.2 0.2 0.2] set trigger box sizes
  (Components|Box|SetBoxExtent (Variables|Default|GetTriggerBox) (/ (Variables|Default|GetTriggerZone) 2.0) true)
  (Transformation|SetRelativeScale3D (Variables|Default|GetCubeIllusionary) (Math|Vector|MakeVector (/ (.x (Variables|Default|GetTriggerZone)) 1e+02) (/ (.y (Variables|Default|GetTriggerZone)) 1e+02) (/ (.z (Variables|Default|GetTriggerZone)) 1e+02)))
  ;[0.2 0.2 0.2] set non-center location and scale
  (Transformation|SetRelativeLocation _triggerbox (/ (Variables|Default|GetTriggerZone) 2.0) false false)
  (Transformation|SetRelativeLocation (Variables|Default|GetCubeIllusionary) (/ (Variables|Default|GetTriggerZone) 2.0) false false)
  (Transformation|SetRelativeScale3D _triggerbox (Math|Vector|MakeVector 1.0 1.0 1.0)))
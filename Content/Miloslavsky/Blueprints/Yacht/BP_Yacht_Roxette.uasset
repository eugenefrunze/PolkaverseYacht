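; Themed yacht actor that, after a delay on activation, either launches a jetski or sails a spline path.
; Construction applies a data table or custom color to hull, garage door and physics-disabled child jetskis.
; BeginPlay optionally spawns an attached, themed helicopter; Autostart (jetski launch) only runs within that branch.
; Launch animates door, platform and cranes before enabling boat physics; sailing runs a length-scaled timeline from spline end to start.
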(event Custom|SailAlongPathSpline
  (bind _pathspline (Variables|MOVEMENT|GetPathSpline))
  ;[0 0 0] Sail along spline path
  ;;[1 0 0.08333] Sail along path
  (Utilities|IsValid (Variables|MOVEMENT|GetNavigationPath)
    (:Is%20Valid
      ;;[0.2 0.2 0.2 1 14] define play rate depends on the path length (to move with specified speed)
      (Components|Timeline|SetPlayRate (Variables|Default|GetTL_MovingAlongPath) (/ (Variables|MOVEMENT|GetSpeed) (/ (Spline|GetSplineLength (Variables|MOVEMENT|GetPathSpline)) 1e+02)))
      (bind _alpha (Timeline|TL_MovingAlongPath PlayFromStart)
        (:Update
          (Transformation|SetActorLocationAndRotation (Spline|GetLocationatDistanceAlongSpline _pathspline (Math|Float|Lerp (Spline|GetSplineLength (Variables|MOVEMENT|GetPathSpline)) 0.0 _alpha) "World") (Spline|GetRotationatDistanceAlongSpline _pathspline (Math|Float|Lerp (Spline|GetSplineLength (Variables|MOVEMENT|GetPathSpline)) 0.0 _alpha) "Local")))))))

(event Custom|LaunchChildBoat
  (bind _jetskies (Variables|JETSKI|GetJetSkies))
  (bind _boatcrane_l (Variables|Default|GetBoatCrane_L))
  (bind _returnvalue (Transformation|GetSocketTransform _boatcrane_l "Socket_BeamLast_01" "RTS_World"))
  (bind _returnvalue_2 (Transformation|GetSocketTransform _boatcrane_l "Socket_BeamLast_02" "RTS_World"))
  ;[0 0 0 1 14] Define the boat to launch (may be changed if boats count changes)
  ;;[1 0 0.08333] Launch child boat
  (if (Utilities|Set|IsNotEmpty _jetskies)
    (bind _result (Utilities|Set|ToArray _jetskies))
    (bind _asbp_boat_base (Utilities|Casting|CastToBP_BoatBase (Variables|/Script/Engine.ChildActorComponent|GetChildActor (Utilities|Array|Get(acopy) _result))))
    ;[0 0 0] Launch the child boat
    ;;[0.2 0.2 0.2] Attach boat mesh to the 1st socket
    (Transformation|AttachComponentToComponent (Variables|/Game/Miloslavsky/Blueprints/BP_BoatBase.BP_BoatBase_C|GetBoatBody _asbp_boat_base) (Variables|Default|GetBoatCrane_L) "Socket_BeamLast_01" "KeepRelative" "KeepRelative" "KeepRelative" true)
    ;;[0.2 0.2 0.2] Play garage door anim
    (CallFunction|OpenDoorSternGarage 0.6)
    ;;[0.2 0.2 0.2] Play platform animation
    (CallFunction|PlayAnimationwithRate 0 0.6 (Variables|Default|GetPlatformStern) false)
    (Utilities|FlowControl|Delay 1.5)
    ;;[0.2 0.2 0.2] Open cranes animation
    (CallFunction|PlayAnimationwithRate 0 0.4 (Variables|Default|GetBoatCrane_L) false)
    (CallFunction|PlayAnimationwithRate 0 0.4 (Variables|Default|GetBoatCrane_R) false)
    (Utilities|FlowControl|Delay 3.0)
    ;;[0.2 0.2 0.2] Move from 1st crane socket to the 2nd
    (Components|Timeline|SetPlayRate (Variables|Default|GetMoveToWaterLevel) 0.3)
    (bind _alpha (Timeline|MoveToWaterLevel PlayFromStart)
      (:Update
        (Transformation|SetWorldLocationAndRotation (Variables|/Game/Miloslavsky/Blueprints/BP_BoatBase.BP_BoatBase_C|GetBoatBody _asbp_boat_base) (.location (Math|Transform|Lerp(Transform) (Math|Transform|MakeTransform (.location _returnvalue) (.rotation _returnvalue) "1.000000,1.000000,1.000000") (Math|Transform|MakeTransform (.location _returnvalue_2) (.rotation _returnvalue_2) "1.000000,1.000000,1.000000") _alpha)) (.rotation (Math|Transform|Lerp(Transform) (Math|Transform|MakeTransform (.location _returnvalue) (.rotation _returnvalue) "1.000000,1.000000,1.000000") (Math|Transform|MakeTransform (.location _returnvalue_2) (.rotation _returnvalue_2) "1.000000,1.000000,1.000000") _alpha)) false false))
      (:Finished
        ;;[0.2 0.2 0.2] Detach from crane socket and simulate physics
        (Transformation|DetachFromComponent (Variables|/Game/Miloslavsky/Blueprints/BP_BoatBase.BP_BoatBase_C|GetBoatBody _asbp_boat_base) "KeepWorld" "KeepWorld" "KeepRelative" true)
        (Physics|SetSimulatePhysics (Variables|/Game/Miloslavsky/Blueprints/BP_BoatBase.BP_BoatBase_C|GetBoatBody _asbp_boat_base) true)))))

(event EventBeginPlay
  ;[1 0 0.08333] Begin play
  ;[0 0 0] Initialization
  ;;[0.2 0.2 0.2] Spawn helicopter at start
  (if (Variables|HELICOPTER|GetHasHelicopter)
    (bind _returnvalue (Game|SpawnActorfromClass "/Game/Miloslavsky/Blueprints/BP_Helicopter_02.BP_Helicopter_02_C" (Variables|HELICOPTER|GetHelicopterLocation) "AlwaysSpawn" "OverrideRootScale" 0 0))
    (bind _output_get (Variables|Default|SetHelicopter _returnvalue))
    (Transformation|AttachActorToActor _output_get self "None" "KeepRelative" "KeepRelative" "KeepRelative" true)
    ;;[0.6418 1 0.3699] Set theme to Helicopter
    (bind _returnvalue_2 (Utilities|GetDataTableRow "/Game/Miloslavsky/Blueprints/Yacht/BR_DT_YachThemes_Data.BR_DT_YachThemes_Data" (Utilities|String|StringToName (Utilities|String|EnumtoString (Variables|THEME|GetYachtThemeName))))
      (:then
        (Default|SetTheme (Variables|Default|GetHelicopter) (select (Variables|THEME|GetUseCustomColor) (Variables|THEME|GetYachtCustomColor) (.color _returnvalue_2)))
        ;[0 0 0] Autoactivate
        (if (Variables|YACHTGENERAL|GetAutostart)
          (CallFunction|OnActivation))))))

(event EventOnActivation
  (params (Activator :type Actor%20Object%20Reference) (Preceding :type Actor%20Object%20Reference) (ActivationType :type Byte :default 0))
  ;[0 0 0] Yacht activities
  ;;[1 0 0.08333] OnActivation
  (Utilities|FlowControl|Delay (Variables|YACHTGENERAL|GetDelayBeforeActivation))
  (switch Utilities|FlowControl|Switch|SwitchonBPE_YachtActivationTypes (Utilities|Enum|ByteToEnumBPE_YachtActivationTypes ActivationType)
    (:NewEnumerator0
      (CallFunction|LaunchChildBoat))
    (:NewEnumerator1
      (CallFunction|SailAlongPathSpline))))

(fn ConstructionScript
  (bind _navigationpath (Variables|MOVEMENT|GetNavigationPath))
  (Utilities|FlowControl|Sequence
    (:then_0
      ;[0 0 0] Set yacht theme
      ;;[0.2 0.2 0.2 1 14] select theme from table of yacht themes
      (bind _returnvalue (Utilities|GetDataTableRow "/Game/Miloslavsky/Blueprints/Yacht/BR_DT_YachThemes_Data.BR_DT_YachThemes_Data" (Utilities|String|StringToName (Utilities|String|EnumtoString (Variables|THEME|GetYachtThemeName))))
        (:then
          ;;[0.2 0.2 0.2 1 14] set yacht body theme or color
          (Utilities|SetThemeColortoMaterial (Variables|Default|GetYacht_Body) 5 "BaseColor" (select (Variables|THEME|GetUseCustomColor) (Variables|THEME|GetYachtCustomColor) (.color _returnvalue))
            (:Output
              (Utilities|SetThemeColortoMaterial (Variables|Default|GetDoor_SternGarage) 1 "BaseColor" (select (Variables|THEME|GetUseCustomColor) (Variables|THEME|GetYachtCustomColor) (.color _returnvalue))
                (:Output
                  ;;[0.2 0.2 0.2 1 14] Add jetski and set theme parameters to it (color etc)
                  (CallFunction|AddJetskiChildActor (select (Variables|THEME|GetUseCustomColor) (Variables|THEME|GetYachtCustomColor) (.color _returnvalue)) (Variables|JETSKI|GetJetskisNumber) (Variables|JETSKI|GetJetskiesTransforms)))))))))
    (:then_1
      ;[0 0 0] Set path spline from bp_pathSpline
      (Utilities|IsValid _navigationpath
        (:Is%20Valid
          (Variables|MOVEMENT|SetPathSpline (Variables|/Game/Miloslavsky/Blueprints/BP_PathSpline.BP_PathSpline_C|GetSpline_Path _navigationpath)))))
    (:then_2
      ;[0 0 0] Attach collision mesh to stern platform
      (Transformation|AttachComponentToComponent (Variables|Default|GetCol_SternPlatform) (Variables|Default|GetPlatformStern) "Socket_BoneSternBase" "KeepRelative" "KeepRelative" "KeepRelative" true))))

(fn AddJetskiChildActor
  (params (Color :type Linear%20Color%20Structure%20%28by%20ref%29) (JetskiNumber :type Integer%20%28by%20ref%29) (JetskiTransforms :type Array%20of%20Transforms))
  ;[0 0 0 1 14] Check if specified jetskies number more than 0
  (if (Math|Conversions|ToBoolean(Integer) JetskiNumber)
    ;[0 0 0 1 14] Add specified number of jetski child actors in a loop
    (for _index (range 0 (- JetskiNumber 1))
      (bind _returnvalue (AddComponent|AddChildActorComponent false (Utilities|Array|Get(acopy) JetskiTransforms _index)))
      (bind _asbp_boat_base (Utilities|Casting|CastToBP_BoatBase (Variables|/Script/Engine.ChildActorComponent|GetChildActor _returnvalue)))
      ;[0.6418 1 0.3699] IsOnTheYacht
      (Variables|/Game/Miloslavsky/Blueprints/BP_BoatBase.BP_BoatBase_C|SetIsOnTheYacht _asbp_boat_base true)
      ;[0 0 0 1 14] Disable physics so jetski will follow the yacht (not to drop into the ocean)
      (Physics|SetSimulatePhysics (Variables|/Game/Miloslavsky/Blueprints/BP_BoatBase.BP_BoatBase_C|GetBoatBody _asbp_boat_base) false)
      ;[0 0 0 1 14] Set yacht theme to the jetski
      (Default|SetTheme _asbp_boat_base Color)
      ;[0 0 0 1 14] Add new jetski to the jetskies set
      (Utilities|Set|Add (Variables|JETSKI|GetJetSkies) _returnvalue))))

(fn OpenDoorSternGarage
  (params (AnimationRate :type Float%20%28double-precision%29))
  (bind _door_sterngarage (Variables|Default|GetDoor_SternGarage))
  (Components|Timeline|SetPlayRate _door_sterngarage AnimationRate)
  (Audio|Components|Audio|Play _door_sterngarage false))

(fn PlayAnimationwithRate
  (params (AnimationIndex :type Integer) (Rate :type Float%20%28double-precision%29) (Mesh :type Skeletal%20Mesh%20Component%20Object%20Reference) (Looping :type Boolean))
  (Components|Timeline|SetPlayRate Mesh Rate)
  (Audio|Components|Audio|Play Mesh Looping))